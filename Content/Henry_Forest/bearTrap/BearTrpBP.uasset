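; Bear trap actor that snaps shut on the first-person character and holds them until they mash E to escape.
; Overlapping the box centres and immobilises the player, enables input on the trap and plays a timeline rotating both claws.
; Reaching the required presses restores walking, reverses the timeline and re-arms the box after a delay.
; A retriggerable delay on key release resets the press count when mashing pauses.
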(event OnComponentBeginOverlap(Box)
  (params (OverlappedComponent :type Primitive%20Component%20Object%20Reference) (OtherActor :type Actor%20Object%20Reference) (OtherComp :type Primitive%20Component%20Object%20Reference) (OtherBodyIndex :type Integer) (bFromSweep :type Boolean) (SweepResult :type Hit%20Result%20Structure%20%28by%20ref%29))
  (bind _asfirst_person_character (Utilities|Casting|CastToFirstPersonCharacter OtherActor))
  (CallFunction|CatchPlayer _asfirst_person_character)
  (Input|EnableInput (Game|GetPlayerController 0))
  (Collision|SetCollisionEnabled (Variables|Default|GetBox) "NoCollision")
  (bind _track1 (Timeline|Open/Close%20Bear%20Trap Play)
    (:Update
      (Transformation|SetRelativeRotation (Variables|Default|GetRight%20Claw) (Math|Rotator|MakeRotator 0.0 (Math|Float|Lerp 0.0 1.5e+02 _track1) 0.0) false false)
      (Transformation|SetRelativeRotation (Variables|Default|GetLeft%20Claw) (Math|Rotator|MakeRotator 0.0 (Math|Float|Lerp 0.0 -1.5e+02 _track1) 0.0) false false))))

(event Custom|Catch%20Player
  (params (Character :type Character%20Object%20Reference))
  (bind _box (Variables|Default|GetBox))
  (bind _returnvalue (Transformation|GetWorldLocation _box))
  (Pawn|Components|CharacterMovement|DisableMovement (Variables|/Script/Engine.Character|GetCharacterMovement Character))
  (Transformation|SetActorLocation Character (Math|Vector|MakeVector (.x _returnvalue) (.y _returnvalue) (.z (Transformation|GetActorLocation Character))) false false))

(event Custom|Open
  (Pawn|Components|CharacterMovement|SetMovementMode (Variables|/Script/Engine.Character|GetCharacterMovement (stale OnComponentBeginOverlap(Box) _asfirst_person_character)) "MOVE_Walking" 0)
  (Utilities|FlowControl|Sequence
    (:then_0
      (bind _track1 (Timeline|Open/Close%20Bear%20Trap Reverse)
        (:Update
          (Transformation|SetRelativeRotation (Variables|Default|GetRight%20Claw) (Math|Rotator|MakeRotator 0.0 (Math|Float|Lerp 0.0 1.5e+02 _track1) 0.0) false false)
          (Transformation|SetRelativeRotation (Variables|Default|GetLeft%20Claw) (Math|Rotator|MakeRotator 0.0 (Math|Float|Lerp 0.0 -1.5e+02 _track1) 0.0) false false))))
    (:then_1
      (Utilities|FlowControl|Delay 3.0)
      (Collision|SetCollisionEnabled (Variables|Default|GetBox) "QueryAndPhysics")
      (Development|PrintString "1"))))

(event Input|KeyboardEvents|E
  (params (Key :type Key%20Structure))
  (:Pressed
    (bind _result (Math|Integer|IncrementInt (Variables|Default|GetPresses))
      (:%20%20
        (if (== _result (Variables|Default|GetPresses%20Needed))
          (CallFunction|Open)))))
  (:Released
    (Utilities|FlowControl|RetriggerableDelay 0.5)
    (Variables|Default|SetPresses 0)))

(fn ConstructionScript)