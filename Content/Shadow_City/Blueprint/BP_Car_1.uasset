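; BP_Car_1 is an AI-driven car that patrols a looping route and respawns the player when hit.
; Chained AIMoveTo calls visit four waypoints, and the Patrol event restarts the chain; a failed move ends the loop.
; When FirstPersonCharacter overlaps component E, delayed camera fades hide a teleport to the character's Respawn location, then PlayerHunger is set to full.
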(event OnComponentBeginOverlap(e)
  (params (OverlappedComponent :type Primitive%20Component%20Object%20Reference) (OtherActor :type Actor%20Object%20Reference) (OtherComp :type Primitive%20Component%20Object%20Reference) (OtherBodyIndex :type Integer) (bFromSweep :type Boolean) (SweepResult :type Hit%20Result%20Structure%20%28by%20ref%29))
  (bind _returnvalue (Game|GetPlayerCameraManager 0))
  (bind _asfirst_person_character (Utilities|Casting|CastToFirstPersonCharacter OtherActor))
  (Utilities|FlowControl|Delay 1.0)
  (CameraFades|StartCameraFade :self _returnvalue :ToAlpha 1.0 :Duration 1.0 :bHoldWhenFinished true)
  (Utilities|FlowControl|Delay 1.0)
  (Transformation|SetActorTransform _asfirst_person_character (Math|Transform|MakeTransform (Math|Vector|MakeVector (.x (Variables|/Game/Henry_Forest/FirstPersonBP/Blueprints/FirstPersonCharacter.FirstPersonCharacter_C|GetRespawn _asfirst_person_character)) (.y (Variables|/Game/Henry_Forest/FirstPersonBP/Blueprints/FirstPersonCharacter.FirstPersonCharacter_C|GetRespawn _asfirst_person_character)) (.z (Variables|/Game/Henry_Forest/FirstPersonBP/Blueprints/FirstPersonCharacter.FirstPersonCharacter_C|GetRespawn _asfirst_person_character))) "0, 0, 0" "1,1,1"))
  (Utilities|FlowControl|Delay 1.0)
  (CameraFades|StartCameraFade :self _returnvalue :FromAlpha 1.0 :Duration 2.0 :bHoldWhenFinished true)
  (Variables|/Game/Henry_Forest/FirstPersonBP/Blueprints/FirstPersonCharacter.FirstPersonCharacter_C|SetplayerHunger _asfirst_person_character 100))

(event Custom|Patrol
  (bind _self self)
  (AI|AIMoveTo _self "0, 0, 0" (Variables|Default|GetWaypoint1) 5.0 false
    (:OnSuccess
      (AI|AIMoveTo _self "0, 0, 0" (Variables|Default|GetWaypoint2) 5.0 false
        (:OnSuccess
          (AI|AIMoveTo _self "0, 0, 0" (Variables|Default|GetWaypoint3) 5.0 false
            (:OnSuccess
              (AI|AIMoveTo _self "0, 0, 0" (Variables|Default|GetWaypoint4) 5.0 false
                (:OnSuccess
                  (CallFunction|Patrol))))))))))

(event EventBeginPlay
  (bind _self self)
  (AI|AIMoveTo _self "0, 0, 0" (Variables|Default|GetWaypoint1) 5.0 false
    (:OnSuccess
      (AI|AIMoveTo _self "0, 0, 0" (Variables|Default|GetWaypoint2) 5.0 false
        (:OnSuccess
          (AI|AIMoveTo _self "0, 0, 0" (Variables|Default|GetWaypoint3) 5.0 false
            (:OnSuccess
              (AI|AIMoveTo _self "0, 0, 0" (Variables|Default|GetWaypoint4) 5.0 false
                (:OnSuccess
                  (CallFunction|Patrol))))))))))

(fn ConstructionScript)